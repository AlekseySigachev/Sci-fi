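; Game mode for a multiplayer star-map game: spawns players and their ships at the start station and cycles a single controller's possession between them.
; Players and ships move separately; the HUD Move button reflects whether the ship's star allows that one-cell grid direction.
; Ship moves reshuffle orbits and discover the destination star.
; Entering a star uses SolarSystemBuilder's sub-scene copy; exiting looks up the original in MapBuilder's dictionary.
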(event `self.ReceiveBeginPlay`
  (set `self.PlayerController` (cast `/Game/Blueprints/Controlls/BP_MainController` (`GameplayStatics.GetPlayerController` 0) :!pure true))
  (bind _returnvalue (`GameplayStatics.GetActorOfClass` "/Game/Blueprints/BP_SpaceObject_Station.BP_SpaceObject_Station_C"))
  (bind _output_get (set `self.StartStation` _returnvalue))
  (`self.SpawnPlayers` _output_get)
  (bind _returnvalue_2 (`|CreateWidget` "/Game/ProjectS/UI/HUD.HUD_C"))
  (bind _output_get_2 (set `self.HUD` _returnvalue_2))
  (`UserWidget.AddToViewport` _output_get_2 0)
  (for (_array_element _array_index) (`self.Players`)
    (`self.K2_SetActorLocation` _array_element (`|GetArrayItem` (`/Game/Blueprints/BP_SpaceObject.Posititons` (`self.StartStation`)) _array_index) false false))
  (`self.DrawScene`))

(fn `CheckAllowedDirection`
  (params (ShipStar :type "/Game/Blueprints/BP_SpaceObject Object Reference") (PlayerStar :type "/Game/Blueprints/BP_SpaceObject Object Reference"))
  (locals (CheckableDirection :type Integer) (HorizontalMove :type Boolean) (TopDownMove :type Boolean))
  (bind _direction_list (`/Game/Blueprints/BP_SpaceObject.get_allow_direction_list` ShipStar))
  (bind _direction (`self.GetRequieredDirection` (`local.PlayerStar`) (`local.ShipStar`)))
  (`self.On_Off_MoveButton` (`KismetArrayLibrary.Array_IsValidIndex` _direction_list (`KismetArrayLibrary.Array_Find` _direction_list _direction))))

(fn `CreateStarCopy`
  (params (Scene :type "Actor Object Reference") (Star :type "/Game/Blueprints/BP_SpaceObject Object Reference"))
  (returns (StarCopy :type "/Game/Blueprints/BP_SpaceObject Object Reference"))
  (locals (Copy :type "/Game/Blueprints/BP_SpaceObject Object Reference"))
  (bind _returnvalue_location (`KismetMathLibrary.BreakTransform` (`self.GetTransform` Scene)))
  (bind _star (`local.Star`))
  (bind _returnvalue (`|SpawnActorFromClass` (`GameplayStatics.GetObjectClass` Star) (`KismetMathLibrary.MakeTransform` _returnvalue_location (struct) (0.05 0.05 0.05)) "Undefined" "OverrideRootScale" null 0 0 0 (`/Game/Blueprints/BP_SpaceObject.name` Star) true true null))
  (set `local.Copy` _returnvalue)
  (set `/Game/Blueprints/BP_SpaceObject.m_pos_x` (`/Game/Blueprints/BP_SpaceObject.m_pos_x` _star) (`local.Copy`))
  (set `/Game/Blueprints/BP_SpaceObject.m_pos_y` (`/Game/Blueprints/BP_SpaceObject.m_pos_y` _star) (`local.Copy`))
  (return (`local.Copy`)))

(fn `DrawScene`
  (locals (Delta :type "Vector Structure" :default (600.0 0.0 0.0)))
  (bind _returnvalue_location (`KismetMathLibrary.BreakTransform` (`self.GetTransform` (`self.StartStation`))))
  (bind _returnvalue (`|SpawnActorFromClass` "/Game/Blueprints/Map/BP_Scene.BP_Scene_C" (`KismetMathLibrary.MakeTransform` _returnvalue_location) "Undefined" "OverrideRootScale" null null))
  (bind _output_get (set `self.MainScene` _returnvalue))
  (bind _returnvalue_2 (`|SpawnActorFromClass` "/Game/Blueprints/Map/BP_Sub_Scene.BP_Sub_Scene_C" (`KismetMathLibrary.MakeTransform` (+ (`self.K2_GetActorLocation` _output_get) (`local.Delta`))) "Undefined" "OverrideRootScale" null null))
  (bind _returnvalue_3 (`|SpawnActorFromClass` "/Game/Blueprints/Map/BP_SolarSystemBuilder.BP_SolarSystemBuilder_C" (`KismetMathLibrary.MakeTransform` (0.0 0.0 0.0)) "Undefined" "OverrideRootScale" null _returnvalue_2 null))
  (set `self.SolarSystemBuilder` _returnvalue_3))

(fn `GetPlayerQuantity`
  (returns (PlayersQuantity :type Integer))
  (return (`/Game/Blueprints/Controlls/BP_MainGameInstance.PlayersQuantity` (cast `/Game/Blueprints/Controlls/BP_MainGameInstance` (`GameplayStatics.GetGameInstance`) :!pure true))))

(fn `GetRequieredDirection`
  (params (PlayerStar :type "/Game/Blueprints/BP_SpaceObject Object Reference") (ShipStar :type "/Game/Blueprints/BP_SpaceObject Object Reference"))
  (returns (Direction :type Integer))
  (locals (PlayerStarLocation :type "Vector Structure" :default (0.0 0.0 0.0)) (ShipStarLocation :type "Vector Structure" :default (0.0 0.0 0.0)) (LDirection :type Integer))
  (bind _grid_step (`/Game/Blueprints/BP_SpaceObject.get_grid_step` (`local.PlayerStar`)))
  (bind (_returnvalue_x _returnvalue_y) (`KismetMathLibrary.BreakVector` (- (`local.ShipStarLocation`) (`local.PlayerStarLocation`))))
  (bind (_returnvalue_x_2 _returnvalue_y_2) (`KismetMathLibrary.BreakVector` (- (`local.ShipStarLocation`) (`local.PlayerStarLocation`))))
  (bind _returnvalue (== _returnvalue_x 0.0))
  (bind _returnvalue_2 (== _returnvalue_y 0.0))
  (set `local.LDirection` 0)
  (set `local.PlayerStarLocation` (`self.K2_GetActorLocation` (`local.PlayerStar`)))
  (set `local.ShipStarLocation` (`self.K2_GetActorLocation` (`local.ShipStar`)))
  (if (!= (`local.ShipStarLocation`) (`local.PlayerStarLocation`))
    (if (not (or (== (`KismetMathLibrary.Abs` (/ _returnvalue_x_2 _grid_step)) 1.0) (== (`KismetMathLibrary.Abs` (/ _returnvalue_y_2 _grid_step)) 1.0)))
      _
      (elif (and (not _returnvalue) (not _returnvalue_2))
        _
        (else
          (`|ExecutionSequence`
            (:`then_0`
              (if _returnvalue
                (bind _output_get (`self.IsTopDownMove` (`local.ShipStarLocation`) (`local.PlayerStarLocation`)))
                (set `local.LDirection` _output_get)
                (else
                  (bind _output_get_2 (`self.IsLeftRightMove` (`local.ShipStarLocation`) (`local.PlayerStarLocation`)))
                  (set `local.LDirection` _output_get_2))))
            (:`then_2`
              (if _returnvalue_2
                (bind _output_get_3 (`self.IsLeftRightMove` (`local.ShipStarLocation`) (`local.PlayerStarLocation`)))
                (set `local.LDirection` _output_get_3)
                (else
                  (bind _output_get_4 (`self.IsTopDownMove` (`local.ShipStarLocation`) (`local.PlayerStarLocation`)))
                  (set `local.LDirection` _output_get_4)))))
          (return (`local.LDirection`)))))
    (return (`local.LDirection`))))

(fn `GoInsideStar`
  (locals (ThisStar :type "/Game/Blueprints/BP_SpaceObject Object Reference") (StarCopy :type "/Game/Blueprints/BP_SpaceObject Object Reference") (IsSameLocations :type Boolean))
  (bind (_issamelocation _star) (`self.IsSameLocation`))
  (set `local.ThisStar` _star)
  (set `local.IsSameLocations` _issamelocation)
  (bind _cangoinside (`/Game/Blueprints/BP_SpaceObject.CanGoInside` (`local.ThisStar`)))
  (if _cangoinside
    (bind _starcopy (`/Game/Blueprints/Map/BP_SolarSystemBuilder.BuildSolarSystem` (`self.SolarSystemBuilder`) (`local.ThisStar`)))
    (set `local.StarCopy` _starcopy)
    (`self.MoveToLocation` (`local.IsSameLocations`) (`local.StarCopy`))))

(fn `GoOutSideStar`
  (locals (ThisStar :type "/Game/Blueprints/BP_SpaceObject Object Reference"))
  (bind _currentstar (`/Game/Blueprints/Controlls/BP_Player.CurrentStar` (`self.CurrentPlayer`)))
  (bind _mapbuilder (`/Game/Blueprints/BP_SpaceObject.MapBuilder` _currentstar))
  (bind _new_key (`/Game/Blueprints/Map/BP_MapBuilder.gen_new_key` _mapbuilder (`/Game/Blueprints/BP_SpaceObject.m_pos_x` _currentstar) (`/Game/Blueprints/BP_SpaceObject.m_pos_y` _currentstar)))
  (bind (_value _returnvalue) (`BlueprintMapLibrary.Map_Find` (`/Game/Blueprints/Map/BP_MapBuilder.m_mase_dict` _mapbuilder) _new_key))
  (if _returnvalue
    (bind _issamelocation (`self.IsSameLocation`))
    (`self.MoveToLocation` _issamelocation _value)))

(fn `IsLeftRightMove`
  (params (LShipLoc :type "Vector Structure") (LPlayerLoc :type "Vector Structure"))
  (returns (Output_Get :type Integer))
  (locals (LDirection :type Integer))
  (if (> (- LShipLoc_X LPlayerLoc_X) 0.0)
    (bind _output_get (set `local.LDirection` 2))
    (return _output_get)
    (else
      (bind _output_get_2 (set `local.LDirection` 8))
      (return _output_get_2))))

(fn `IsSameLocation`
  (returns (IsSameLocation :type Boolean) (Star :type "/Game/Blueprints/BP_SpaceObject Object Reference"))
  (locals (IsSameLocations :type Boolean) (ThisStar :type "/Game/Blueprints/BP_SpaceObject Object Reference"))
  (bind _currentplayer (`self.CurrentPlayer`))
  (bind _currentstar (`/Game/Blueprints/Controlls/BP_Player.CurrentStar` _currentplayer))
  (bind _output_get (set `local.ThisStar` _currentstar))
  (bind _output_get_2 (set `local.IsSameLocations` (== _currentstar (`/Game/Blueprints/Controlls/BP_PlayerShip.CurrentStar` (`/Game/Blueprints/Controlls/BP_Player.Ship` _currentplayer)))))
  (return _output_get_2 _output_get))

(fn `IsTopDownMove`
  (params (LShipLoc :type "Vector Structure") (LPlayerLoc :type "Vector Structure"))
  (returns (Output_Get :type Integer))
  (locals (LDirection :type Integer))
  (if (< (- LShipLoc_Y LPlayerLoc_Y) 0.0)
    (bind _output_get (set `local.LDirection` 1))
    (return _output_get)
    (else
      (bind _output_get_2 (set `local.LDirection` 4))
      (return _output_get_2))))

(fn `Move Ship to Location`
  (locals (DestStar :type "/Game/Blueprints/BP_SpaceObject Object Reference") (SourceStar :type "/Game/Blueprints/BP_SpaceObject Object Reference"))
  (bind _currentplayer (`self.CurrentPlayer`))
  (bind _ship (`/Game/Blueprints/Controlls/BP_Player.Ship` _currentplayer))
  (set `local.DestStar` (`/Game/Blueprints/Controlls/BP_Player.CurrentStar` _currentplayer))
  (set `local.SourceStar` (`/Game/Blueprints/Controlls/BP_PlayerShip.CurrentStar` _ship))
  (set `/Game/Blueprints/Controlls/BP_PlayerShip.CurrentStar` (`local.DestStar`) _ship)
  (`/Game/Blueprints/BP_SpaceObject.AddSpaceObjectToOrbit` (`local.DestStar`) _ship)
  (`/Game/Blueprints/BP_SpaceObject.CalcObjectPositionOnOrbit` (`local.DestStar`))
  (`/Game/Blueprints/BP_SpaceObject.ReallocateObjectsOnOrbit` (`local.DestStar`))
  (`/Game/Blueprints/BP_SpaceObject.RemoveObjectFromOrbit` (`local.SourceStar`) _ship)
  (`/Game/Blueprints/BP_SpaceObject.CalcObjectPositionOnOrbit` (`local.SourceStar`))
  (`/Game/Blueprints/BP_SpaceObject.ReallocateObjectsOnOrbit` (`local.SourceStar`))
  (`/Game/Blueprints/BP_SpaceObject.DiscoverStar` (`local.DestStar`))
  (`self.ToggleInsideButton` (`local.DestStar`)))

(fn `MovePlayerToLocation`
  (params (Target :type "/Game/Blueprints/BP_SpaceObject Object Reference"))
  (bind _currentplayer (`self.CurrentPlayer`))
  (bind _currentplayer_2 (`self.CurrentPlayer`))
  (bind (_returnvalue_x _returnvalue_y) (`KismetMathLibrary.BreakVector` (`self.K2_GetActorLocation` (`/Game/Blueprints/Controlls/BP_Player.CurrentStar` _currentplayer_2))))
  (`self.ToggleInsideButton` Target)
  (set `/Game/Blueprints/Controlls/BP_Player.CurrentStar` (`local.Target`) (`self.CurrentPlayer`))
  (`self.K2_SetActorLocation` _currentplayer_2 (`KismetMathLibrary.MakeVector` _returnvalue_x _returnvalue_y) false false)
  (`self.CheckAllowedDirection` (`/Game/Blueprints/Controlls/BP_PlayerShip.CurrentStar` (`/Game/Blueprints/Controlls/BP_Player.Ship` _currentplayer)) (`/Game/Blueprints/Controlls/BP_Player.CurrentStar` _currentplayer)))

(fn `MoveToLocation`
  (params (IsSameLocation :type Boolean) (Target :type "/Game/Blueprints/BP_SpaceObject Object Reference"))
  (if IsSameLocation
    (`self.MovePlayerToLocation` Target)
    (`self.Move Ship to Location`)
    (else
      (`self.MovePlayerToLocation` Target))))

(fn `PossesNextPlayer`
  (bind _players (`self.Players`))
  (bind _returnvalue (+ (`KismetArrayLibrary.Array_Find` _players (`self.CurrentPlayer`)) 1))
  (if (< _returnvalue (`KismetArrayLibrary.Array_Length` _players))
    (bind _output_get (set `self.CurrentPlayer` (`|GetArrayItem` (`self.Players`) _returnvalue)))
    (`Controller.Possess` (`self.PlayerController`) _output_get)
    (else
      (`self.PossessFirstPlayer`))))

(fn `PossessFirstPlayer`
  (bind _output_get (set `self.CurrentPlayer` (`|GetArrayItem` (`self.Players`))))
  (`Controller.Possess` (`self.PlayerController`) _output_get))

(fn `SpawnPlayers`
  (params (StartStation :type "/Game/Blueprints/BP_SpaceObject_Station Object Reference"))
  (locals (Player :type "/Game/Blueprints/Controlls/BP_Player Object Reference"))
  (bind _player (`local.Player`))
  (bind _player_2 (`local.Player`))
  (bind _startstation (`self.StartStation`))
  (bind _playersquantity (`self.GetPlayerQuantity`))
  (for _ (range 1 (+ _playersquantity 1))
    (bind _returnvalue (`|SpawnActorFromClass` "/Game/Blueprints/Controlls/BP_Player.BP_Player_C" (`KismetMathLibrary.MakeTransform` (0.0 0.0 0.0)) "AlwaysSpawn" "OverrideRootScale" null null))
    (set `local.Player` _returnvalue)
    (`KismetArrayLibrary.Array_Add` (`self.Players`) _player)
    (`/Game/Blueprints/BP_SpaceObject.AddSpaceObjectToOrbit` (`self.StartStation`) (`/Game/Blueprints/Controlls/BP_Player.Ship` _player))
    (set `/Game/Blueprints/Controlls/BP_Player.CurrentStar` (`self.StartStation`) _player_2)
    (set `/Game/Blueprints/Controlls/BP_PlayerShip.CurrentStar` (`self.StartStation`) (`/Game/Blueprints/Controlls/BP_Player.Ship` _player_2)))
  (`self.PossessFirstPlayer`)
  (`/Game/Blueprints/BP_SpaceObject.CalcObjectPositionOnOrbit` _startstation)
  (`/Game/Blueprints/BP_SpaceObject.ReallocateObjectsOnOrbit` _startstation))

(fn `ToggleInsideButton`
  (params (Target :type "/Game/Blueprints/BP_SpaceObject Object Reference"))
  (bind _cangoinside (`/Game/Blueprints/BP_SpaceObject.CanGoInside` Target))
  (bind _discovered (`/Game/Blueprints/BP_SpaceObject.IsDiscovered` Target))
  (`Widget.SetIsEnabled` (`/Game/ProjectS/UI/HUD.GoInside` (`self.HUD`)) (and _discovered _cangoinside)))

(fn `UserConstructionScript`)