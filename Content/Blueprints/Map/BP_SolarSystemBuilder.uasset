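; Map actor that builds a solar system view around a copy of a selected star and animates its orbiting bodies.
; BuildSolarSystem spawns the star copy, reads its planet count from the Sars_system data table, and spawns Circle bodies with OrbitLine rings at stepped radii.
; Once the map is valid, Tick repositions each body through CalcObjectPositionOnOrbit, using sine and cosine of accumulated time on a flat circular orbit.
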(event `self.ReceiveBeginPlay`
  (set `self.ValidMap` false))

(event `self.ReceiveTick`
  (params (DeltaSeconds :type "Float (single-precision)"))
  (bind _orbitalobjects (`self.OrbitalObjects`))
  (set `self.Time` (+ (`self.Time`) (`GameplayStatics.GetWorldDeltaSeconds`)))
  (if (`self.ValidMap`)
    (for _index (range (+ (`KismetArrayLibrary.Array_LastIndex` _orbitalobjects) 1))
      (bind _output (`|GetArrayItem` _orbitalobjects _index))
      (bind _posititon (`self.CalcObjectPositionOnOrbit` 1 (`/Game/Blueprints/Circle.Speed` (cast `/Game/Blueprints/Circle` _output :!pure true)) (+ _index 1) 12 (`self.Star`)))
      (`self.K2_SetActorLocation` _output _posititon false false))))

(fn `BuildSolarSystem`
  (params (Star :type "/Game/Blueprints/BP_SpaceObject Object Reference"))
  (returns (StarCopy :type "/Game/Blueprints/BP_SpaceObject Object Reference"))
  (locals (CopiedStar :type "/Game/Blueprints/BP_SpaceObject Object Reference") (Bodies :type "Array of /Game/Blueprints/Circle Object Reference"))
  (bind _copiedstar (`local.CopiedStar`))
  (bind _bodies (`local.Bodies`))
  (bind (_returnvalue_x _returnvalue_y) (`KismetMathLibrary.BreakVector` (`self.K2_GetActorLocation` (`local.CopiedStar`))))
  (bind _so_copy (`self.CreateStarCopy` Star))
  (bind _output_get (set `self.Star` _so_copy))
  (bind _output_get_2 (set `local.CopiedStar` _output_get))
  (bind _returnvalue (`|GetDataTableRow` "/Game/Data/Sars_system.Sars_system" (`KismetStringLibrary.Conv_StringToName` (`/Game/Blueprints/BP_SpaceObject.name` _output_get_2)))
    (:`then`
      (for _index (range 1 (+ (`.planet_quantity_13_58A3ECE84D5C91AE66C9FFAB78C422F2` (break `/Game/Data/Star_system_struct` _returnvalue)) 1))
        (bind _returnvalue_2 (`|SpawnActorFromClass` "/Game/Blueprints/Circle.Circle_C" (`KismetMathLibrary.MakeTransform` (`KismetMathLibrary.MakeVector` (+ _returnvalue_x (* 12 _index)) _returnvalue_y) (struct) (0.01 0.01 0.01)) "Undefined" "OverrideRootScale" null null))
        (`KismetArrayLibrary.Array_Add` (`local.Bodies`) _returnvalue_2))
      (for _index_2 (range (+ (`KismetArrayLibrary.Array_LastIndex` _bodies) 1))
        (bind _returnvalue_3 (+ _index_2 1))
        (bind _posititon (`self.CalcObjectPositionOnOrbit` 1 (`KismetMathLibrary.RandomFloatInRange` 1.0 50.0) _returnvalue_3 (`/Game/Blueprints/BP_SpaceObject.get_grid_step` _copiedstar) _copiedstar))
        (bind _output (`|GetArrayItem` _bodies _index_2))
        (if (`KismetSystemLibrary.IsValid` _output)
          (`self.K2_SetActorLocation` _output _posititon false false)
          (`self.SpawnLineOrbit` (`self.K2_GetActorLocation` (`local.CopiedStar`)) _returnvalue_3)
          (else
            (`KismetSystemLibrary.PrintString` "Hello"))))
      (set `self.ValidMap` true)
      (set `self.OrbitalObjects` (`local.Bodies`))
      (return (`local.CopiedStar`)))))

(fn `CalcObjectPositionOnOrbit`
  (params (BodyNum :type Integer) (OrbitalSpeed :type "Float (double-precision)") (CellMagnification :type Integer) (CellSize :type Integer) (Star :type "/Game/Blueprints/BP_SpaceObject Object Reference"))
  (returns (Posititon :type "Vector Structure"))
  (locals (step :type "Float (double-precision)") (ContainerPosition :type "Vector Structure" :default (0.0 0.0 0.0)) (Angle :type "Float (double-precision)") (OrbiralRadius :type Integer) (Speed :type "Float (double-precision)") (FirstTime :type Boolean :default true))
  (bind _orbiralradius (`local.OrbiralRadius`))
  (bind (_containerposition_x _containerposition_y) (`KismetMathLibrary.BreakVector` (`local.ContainerPosition`)))
  (set `local.OrbiralRadius` (* CellMagnification CellSize))
  (set `local.ContainerPosition` (`self.K2_GetActorLocation` (`local.Star`)))
  ;[1 1 1] calculate step
  (set `local.step` (/ (* (`KismetMathLibrary.GetPI`) 2.0) (`local.BodyNum`)))
  (for _index (range 1 (+ (`local.BodyNum`) 1))
    ;[1 1 1] angle
    (bind _output_get (set `local.Angle` (* _index (`local.step`))))
    (bind _returnvalue (+ (* (`local.Speed`) (`self.Time`)) _output_get))
    (return (`KismetMathLibrary.MakeVector` (+ _containerposition_x (* (`KismetMathLibrary.Cos` _returnvalue) _orbiralradius)) (+ _containerposition_y (* (`KismetMathLibrary.Sin` _returnvalue) _orbiralradius))))))

(fn `CreateStarCopy`
  (params (Star :type "/Game/Blueprints/BP_SpaceObject Object Reference"))
  (returns (SO_Copy :type "/Game/Blueprints/BP_SpaceObject Object Reference"))
  (locals (Copy :type "/Game/Blueprints/BP_SpaceObject Object Reference"))
  (bind _star (`local.Star`))
  (bind _returnvalue_location (`KismetMathLibrary.BreakTransform` (`self.GetTransform` (`self.Scene`))))
  (bind _returnvalue (`|SpawnActorFromClass` (`GameplayStatics.GetObjectClass` Star) (`KismetMathLibrary.MakeTransform` _returnvalue_location (struct) (0.05 0.05 0.05)) "Undefined" "OverrideRootScale" null 0 0 0 (`/Game/Blueprints/BP_SpaceObject.name` Star) true true null))
  (set `local.Copy` _returnvalue)
  (set `/Game/Blueprints/BP_SpaceObject.m_pos_x` (`/Game/Blueprints/BP_SpaceObject.m_pos_x` _star) (`local.Copy`))
  (set `/Game/Blueprints/BP_SpaceObject.m_pos_y` (`/Game/Blueprints/BP_SpaceObject.m_pos_y` _star) (`local.Copy`))
  (return (`local.Copy`)))

(fn `SpawnLineOrbit`
  (params (SpawnTransform_Location :type "Vector Structure") (CellMagnification :type Integer))
  (bind _returnvalue (`|SpawnActorFromClass` "/Game/Blueprints/Map/OrbitLine.OrbitLine_C" (`KismetMathLibrary.MakeTransform` SpawnTransform_Location (struct) (1.0 1.0 0.01)) "Undefined" "OverrideRootScale" null null))
  (`/Game/Blueprints/Map/OrbitLine.SetRadius` _returnvalue CellMagnification))

(fn `UserConstructionScript`)