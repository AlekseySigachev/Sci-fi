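; Builds a grid star map that starts from a spawned station and is revealed through star discovery.
; Objects are keyed by "X_Y" strings, with direction flags (1/2/4/8) giving neighbour offsets where the station spawns undiscovered star placeholders.
; DiscoverStar fills a placeholder with a random row drawn from the Sars_system table pool.
; When the pool empties, unnamed stars are destroyed and arrows to empty cells are disabled.
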(event `self.ReceiveBeginPlay`
  (`self.add_start_station` 15 15 15 "StartStation"))

(fn `add_key_and_history`
  (params (Object :type "/Game/Blueprints/BP_SpaceObject Object Reference (by ref)") (Key :type "String (by ref)"))
  (`BlueprintMapLibrary.Map_Add` (`self.m_mase_dict`) Key Object)
  (`KismetArrayLibrary.Array_Add` (`self.m_object_discovery_history`) Object)
  (return))

(fn `add_start_station`
  (params (direction :type Integer) (pos_x :type Integer) (pos_y :type Integer) (name :type String))
  (bind _m_station (`self.m_station`))
  (bind _returnvalue (`|SpawnActorFromClass` "/Game/Blueprints/BP_SpaceObject_Station.BP_SpaceObject_Station_C" (`KismetMathLibrary.MakeTransform` (0.0 0.0 0.0) (struct) (0.05 0.05 0.05)) "Undefined" "OverrideRootScale" null direction pos_x pos_y name false false null))
  (bind _output_get (set `self.m_station` _returnvalue))
  (`/Game/Blueprints/BP_SpaceObject.OnDiscovered` _output_get)
  (bind _new_key (`self.gen_new_key` (`local.pos_x`) (`local.pos_y`)))
  (`self.add_key_and_history` (`self.m_station`) _new_key)
  (bind _coord (`/Game/Blueprints/BP_SpaceObject.get_coords` _m_station))
  (bind _direction_list (`/Game/Blueprints/BP_SpaceObject.get_allow_direction_list` _m_station))
  (`self.create_undiscovered_stars` _direction_list _coord)
  (return))

(fn `calc_new_delta`
  (params (directions :type Integer))
  (returns (new_delta :type "Vector2D Structure"))
  (locals (delta :type "Vector2D Structure"))
  (switch `string` (`KismetStringLibrary.Conv_IntToString` directions)
    (:`1`
      (set `local.delta` (0.0 1.0)))
    (:`2`
      (set `local.delta` (-1.0 0.0)))
    (:`4`
      (set `local.delta` (0.0 -1.0)))
    (:`8`
      (set `local.delta` (1.0 0.0))))
  (return (`local.delta`)))

(fn `clear_unused_arrows`
  (locals (local_mase_dict :type "Map of String to /Game/Blueprints/BP_SpaceObject Object Reference"))
  (bind _values (`BlueprintMapLibrary.Map_Values` (`self.m_mase_dict`)))
  (`self.delete_undiscovered_stars` _values)
  (for _array_element (`self.m_object_discovery_history`)
    (bind _direction_list (`/Game/Blueprints/BP_SpaceObject.get_allow_direction_list` _array_element))
    (for _array_element_2 _direction_list
      (bind _new_delta (`self.calc_new_delta` _array_element_2))
      (bind _coord (`/Game/Blueprints/BP_SpaceObject.get_coords` _array_element))
      (bind (_returnvalue_x _returnvalue_y) (`KismetMathLibrary.BreakVector2D` (+ _coord _new_delta)))
      (bind _new_key (`self.gen_new_key` (`KismetMathLibrary.FTrunc` _returnvalue_x) (`KismetMathLibrary.FTrunc` _returnvalue_y)))
      (if (not (`.ReturnValue` (`BlueprintMapLibrary.Map_Find` (`self.m_mase_dict`) _new_key)))
        (`/Game/Blueprints/BP_SpaceObject.disable_arrow_and_direction` _array_element _array_element_2)))))

(fn `create_undiscovered_stars`
  (params (allow_direction_list :type "Array of Integer") (Coords :type "Vector2D Structure"))
  (locals (new_pos_x :type Integer :default 0) (new_pos_y :type Integer :default 0))
  (for _array_element allow_direction_list
    (bind _new_delta (`self.calc_new_delta` _array_element))
    (bind (_returnvalue_x _returnvalue_y) (`KismetMathLibrary.BreakVector2D` (+ (`local.Coords`) _new_delta)))
    (set `local.new_pos_x` (`KismetMathLibrary.FTrunc` _returnvalue_x))
    (set `local.new_pos_y` (`KismetMathLibrary.FTrunc` _returnvalue_y))
    (bind _new_key (`self.gen_new_key` (`local.new_pos_x`) (`local.new_pos_y`)))
    (if (not (`.ReturnValue` (`BlueprintMapLibrary.Map_Find` (`self.m_mase_dict`) _new_key)))
      (bind _returnvalue (`|SpawnActorFromClass` "/Game/Blueprints/BP_SpaceObject_Star.BP_SpaceObject_Star_C" (`KismetMathLibrary.MakeTransform` (0.0 0.0 0.0) (struct) (0.05 0.05 0.05)) "Undefined" "OverrideRootScale" null 0 (`local.new_pos_x`) (`local.new_pos_y`) "" false true null))
      (bind _new_key_2 (`self.gen_new_key` (`local.new_pos_x`) (`local.new_pos_y`)))
      (`BlueprintMapLibrary.Map_Add` (`self.m_mase_dict`) _new_key_2 _returnvalue))))

(fn `delete_undiscovered_stars`
  (params (Array :type "Array of /Game/Blueprints/BP_SpaceObject Object Reference"))
  (for _array_element Array
    (if (`KismetStringLibrary.IsEmpty` (`/Game/Blueprints/BP_SpaceObject.name` _array_element))
      (bind _coord (`/Game/Blueprints/BP_SpaceObject.get_coords` _array_element))
      (`self.K2_DestroyActor` _array_element)
      (bind _new_key (`self.gen_new_key` (`KismetMathLibrary.FTrunc` (`KismetMathLibrary.BreakVector2D` _coord)) (`KismetMathLibrary.FTrunc` (`.Y` (`KismetMathLibrary.BreakVector2D` _coord)))))
      (`BlueprintMapLibrary.Map_Remove` (`self.m_mase_dict`) _new_key))))

(fn `discover_star`
  (params (key :type String))
  (locals (new_star :type "/Game/Blueprints/BP_SpaceObject Object Reference"))
  (bind (_id _random_star_name _planet_quantity _type _direction _material) (`self.pop_random_star`))
  (bind _output_get (set `local.new_star` (`BlueprintMapLibrary.Map_Find` (`self.m_mase_dict`) (`local.key`))))
  (`/Game/Blueprints/BP_SpaceObject.set_properties` _output_get (`KismetStringLibrary.Conv_NameToString` _random_star_name) (`KismetMathLibrary.Conv_ByteToInt` _direction) 0 _material)
  (`/Game/Blueprints/BP_SpaceObject.OnDiscovered` (`local.new_star`))
  (`KismetArrayLibrary.Array_Add` (`self.m_object_discovery_history`) (`local.new_star`))
  (bind _is_empry (`self.is_empty` (`self.m_stars`)))
  (if _is_empry
    (`self.clear_unused_arrows`)))

(fn `gen_new_key`
  (params (pos_x :type Integer) (pos_y :type Integer))
  (returns (new_key :type String))
  (return (`KismetTextLibrary.Conv_TextToString` (`|FormatText` "{a}_{b}" pos_x pos_y))))

(fn `get_next_place_coords`
  (locals (l_valid_result :type Boolean) (l_allow_directions :type "Array of Integer"))
  (for _ (`local.l_allow_directions`)
    (if (`local.l_valid_result`)
      (break)
      (elif (== (`KismetArrayLibrary.Array_Length` (`local.l_allow_directions`)) 0)
        _))))

(fn `is_empty`
  (params (stars :type "Array of Name"))
  (returns (is_empry :type Boolean))
  (return (`KismetArrayLibrary.Array_IsEmpty` stars)))

(fn `pop_random_star`
  (returns (id :type Integer) (random_star_name :type Name) (planet_quantity :type Integer) (Type :type Integer) (Direction :type Byte) (Material :type "MaterialInstance Object Reference"))
  (bind _output (`|GetArrayItem` (`self.m_stars`) (`KismetMathLibrary.RandomIntegerInRange` 0 (`KismetArrayLibrary.Array_LastIndex` (`self.m_stars`)))))
  (bind _returnvalue (`|GetDataTableRow` "/Game/Data/Sars_system.Sars_system" _output)
    (:`then`
      (`KismetArrayLibrary.Array_RemoveItem` (`self.m_stars`) _output)
      (bind (_id _name _planet_quantity _type _direction _material) (break `/Game/ProjectS/Data/S_Stars` _returnvalue))
      (return _id (`KismetStringLibrary.Conv_StringToName` _name) _planet_quantity _type _direction _material))))

(fn `UserConstructionScript`
  (bind _outrownames (`DataTableFunctionLibrary.GetDataTableRowNames` "/Game/Data/Sars_system.Sars_system"))
  (set `self.m_stars` _outrownames))