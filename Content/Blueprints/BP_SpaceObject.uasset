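; BP_SpaceObject is a clickable star-map node on a grid; clicking it asks the game mode to move the player there.
; Construction reads name, open material and a direction bitmask from a data table; the bitmask drives four arrows showing allowed moves.
; Discovery functions register the star with BP_MapBuilder and create undiscovered neighbours.
; Each tick spins the center mesh and spaces orbiting objects evenly around it using sine/cosine.
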(event OnClicked(CenterObject)
  (params (TouchedComponent :type Primitive%20Component%20Object%20Reference) (ButtonPressed :type Key%20Structure :default "None"))
  (Default|MovePlayertoLocation (Variables|Default|GetGameMode) self))

(event EventBeginPlay
  (Variables|Default|SetGameMode (.AsBP%20Main%20Game%20Mode (Utilities|Casting|CastToBP_MainGameMode (Game|GetGameMode)))))

(event EventTick
  (params (DeltaSeconds :type Float%20%28single-precision%29))
  (Transformation|AddWorldRotation (Variables|Default|GetCenterObject) "0.100000,0.100000,0.100000" false false)
  (Variables|Default|SetTime (+ (Variables|Default|GetTime) (Utilities|Time|GetWorldDeltaSeconds)))
  (CallFunction|CalcObjectPositiononOrbit)
  (CallFunction|ReallocateObjectsonOrbit))

(fn ConstructionScript
  (Rendering|Material|SetMaterial (Variables|Default|GetCenterObject) 0 (Variables|Default|GetCloseMaterial))
  (if (Variables|Default|GetDiscovered)
    _
    (else
      (CallFunction|Draw)))
  (bind _returnvalue (Actor|GetActorOfClass "/Game/Blueprints/Map/BP_MapBuilder.BP_MapBuilder_C"))
  (Variables|Default|SetMapBuilder _returnvalue)
  (bind _returnvalue_2 (Utilities|GetDataTableRow "/Game/Data/Sars_system.Sars_system" (Utilities|String|StringToName (Variables|Default|Getname)))
    (:then
      (CallFunction|SetProperties (.name _returnvalue_2) (Math|Conversions|ToInteger(Byte) (.direction _returnvalue_2)) (.planet_quantity _returnvalue_2) (.material _returnvalue_2))
      (Rendering|Material|SetMaterial (Variables|Default|GetCenterObject) 0 (Variables|Default|GetOpenMaterial)))))

(fn GetCoords
  (return (Math|Conversions|ToVector2D(IntPoint) (Utilities|Struct|MakeIntPoint (Variables|Default|Getm_pos_x) (Variables|Default|Getm_pos_y)))))

(fn IsCanMoveTop
  (return (== (Utilities|IsCanMove 1) 1)))

(fn IsCanMoveRight
  (return (== (Utilities|IsCanMove 2) 2)))

(fn IsCanMoveDown
  (return (== (Utilities|IsCanMove 4) 4)))

(fn IsCanMoveLeft
  (return (== (Utilities|IsCanMove 8) 8)))

(fn GetGridStep
  (return (Variables|Default|GetGRID_STEP)))

(fn EnableArrowTop
  (Rendering|SetVisibility (Variables|Default|GetArrow_top) true false))

(fn EnableArrowRight
  (Rendering|SetVisibility (Variables|Default|GetArrow_right) true false))

(fn EnableArrowDown
  (Rendering|SetVisibility (Variables|Default|GetArrow_down) true false))

(fn EnableArrowLeft
  (Rendering|SetVisibility (Variables|Default|GetArrow_left) true false))

(fn DisableArrowTop
  (Rendering|SetVisibility (Variables|Default|GetArrow_top) false false))

(fn DisableArrowRight
  (Rendering|SetVisibility (Variables|Default|GetArrow_right) false false))

(fn DisableArrowDown
  (Rendering|SetVisibility (Variables|Default|GetArrow_down) false false))

(fn DisableArrowLeft
  (Rendering|SetVisibility (Variables|Default|GetArrow_left) false false))

(fn DisableArrowandDirection
  (params (direction :type Integer))
  (switch string (Utilities|String|ToString(Integer) direction)
    (:1
      (CallFunction|DisableArrowTop))
    (:2
      (CallFunction|DisableArrowRight))
    (:4
      (CallFunction|DisableArrowDown))
    (:8
      (CallFunction|DisableArrowLeft)))
  (Utilities|DisableDirection direction))

(fn EnableArrowandDirection
  (params (direction :type Integer))
  (switch string (Utilities|String|ToString(Integer) direction)
    (:1
      (CallFunction|EnableArrowTop))
    (:2
      (CallFunction|EnableArrowRight))
    (:4
      (CallFunction|EnableArrowDown))
    (:8
      (CallFunction|EnableArrowLeft)))
  (Utilities|EnableDirection direction))

(fn GetAllowDirectionList
  (Utilities|FlowControl|Sequence
    (:then_0
      (bind _can_move (CallFunction|IsCanMoveTop))
      (if _can_move
        (Utilities|Array|Add (LocalVariables|Getl_direction_list) 1)))
    (:then_1
      (bind _newparam (CallFunction|IsCanMoveRight))
      (if _newparam
        (Utilities|Array|Add (LocalVariables|Getl_direction_list) 2)))
    (:then_2
      (bind _newparam_2 (CallFunction|IsCanMoveDown))
      (if _newparam_2
        (Utilities|Array|Add (LocalVariables|Getl_direction_list) 4)))
    (:then_3
      (bind _newparam_3 (CallFunction|IsCanMoveLeft))
      (if _newparam_3
        (Utilities|Array|Add (LocalVariables|Getl_direction_list) 8)))
    (:then_4
      (return (LocalVariables|Getl_direction_list)))))

(fn DrawArrows
  (Utilities|FlowControl|Sequence
    (:then_0
      (bind _can_move (CallFunction|IsCanMoveTop))
      (if _can_move
        (CallFunction|EnableArrowTop)))
    (:then_1
      (bind _newparam (CallFunction|IsCanMoveRight))
      (if _newparam
        (CallFunction|EnableArrowRight)))
    (:then_2
      (bind _newparam_2 (CallFunction|IsCanMoveDown))
      (if _newparam_2
        (CallFunction|EnableArrowDown)))
    (:then_3
      (bind _newparam_3 (CallFunction|IsCanMoveLeft))
      (if _newparam_3
        (CallFunction|EnableArrowLeft)))))

(fn OnDiscovered
  (CallFunction|DrawArrows)
  (Rendering|Material|SetMaterial (Variables|Default|GetCenterObject) 0 (Variables|Default|GetOpenMaterial)))

(fn Draw
  (Transformation|SetActorLocation (Math|Vector|MakeVector (Math|Conversions|ToFloat(Integer) (|(({2E2CDE98-40D7-BB2E-3CB5-0BB6A59030EC}*{CBF54F76-4D87-5B99-10FB-A2865D6CD170})-({CBF54F76-4D87-5B99-10FB-A2865D6CD170}/2)))) (Math|Conversions|ToFloat(Integer) (|(({EF6CFDEB-48DD-3152-7592-17A721958078}*{CBF54F76-4D87-5B99-10FB-A2865D6CD170})-({CBF54F76-4D87-5B99-10FB-A2865D6CD170}/2)))) 0.0) false false)
  (return))

(fn SetProperties
  (params (name :type String) (direction :type Integer) (planet_quantity :type Integer) (material :type Material%20Instance%20Object%20Reference))
  (Variables|Default|Setm_direction direction)
  (Variables|Default|Setname name)
  (Variables|Default|SetOpenMaterial material))

(fn CalcObjectPositiononOrbit
  (Utilities|Array|Clear (Variables|Default|GetPosititons))
  (LocalVariables|SetContainerPosition (Transformation|GetActorLocation))
  ;[1 1 1] calculate step
  (LocalVariables|Setstep (/ (* (Math|Trig|GetPI) 2.0) (Utilities|Array|Length (Variables|Default|GetCurrentOrbitalObjects))))
  (for _index (range 1 (Utilities|Array|Length (Variables|Default|GetCurrentOrbitalObjects)))
    ;[1 1 1] angle
    (bind _output_get (LocalVariables|SetAngle (* _index (LocalVariables|Getstep))))
    ;[1 1 1] calculate position
    (Utilities|Array|Add (Variables|Default|GetPosititons) (Math|Vector|MakeVector (+ (.x (LocalVariables|GetContainerPosition)) (* (Math|Trig|Cos(Radians) (+ (* (Variables|Default|GetOrbitalSpeed) (Variables|Default|GetTime)) _output_get)) (Variables|Default|GetOrbitalRadius))) (+ (.y (LocalVariables|GetContainerPosition)) (* (Math|Trig|Sin(Radians) (+ (* (Variables|Default|GetOrbitalSpeed) (Variables|Default|GetTime)) _output_get)) (Variables|Default|GetOrbitalRadius))) 0.0))))

(fn AddSpaceObjecttoOrbit
  (params (Object :type BP%20Orbital%20Object%20Object%20Reference%20%28by%20ref%29))
  (Utilities|Array|Add (Variables|Default|GetCurrentOrbitalObjects) Object))

(fn ReallocateObjectsonOrbit
  (for (_array_element _array_index) (Variables|Default|GetCurrentOrbitalObjects)
    (Transformation|SetActorLocation _array_element (Utilities|Array|Get(acopy) (Variables|Default|GetPosititons) _array_index) false false)))

(fn DiscoverStar
  (if (not (Variables|Default|GetDiscovered))
    (if (Utilities|Array|IsEmpty (Variables|Default|Getname))
      (bind _new_key (Default|GenNewKey (Variables|Default|GetMapBuilder) (Variables|Default|Getm_pos_x) (Variables|Default|Getm_pos_y)))
      (Default|DiscoverStar (Variables|Default|GetMapBuilder) _new_key)
      (bind _direction_list (CallFunction|GetAllowDirectionList))
      (bind _coord (CallFunction|GetCoords))
      (Default|CreateUndiscoveredStars (Variables|Default|GetMapBuilder) _direction_list _coord)
      (Variables|Default|SetDiscovered true)
      (return))))

(fn RemoveObjectfromOrbit
  (params (Object :type BP%20Orbital%20Object%20Object%20Reference))
  (Utilities|Array|RemoveItem (Variables|Default|GetPosititons) (Transformation|GetActorLocation Object))
  (Utilities|Array|RemoveItem (Variables|Default|GetCurrentOrbitalObjects) Object))

(fn CanGoInside
  (return (Variables|Default|GetIsInsidable)))

(fn IsDiscovered
  (return (Variables|Default|GetDiscovered)))